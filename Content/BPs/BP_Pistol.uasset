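; BP_Pistol is a pistol weapon that fires, stops firing and reloads through an EBBarrel ballistics component.
; Each shot triggers sound and muzzle FX, and an empty magazine plays a rate-limited out-of-ammo sound.
; Reload blocks shooting during a timed animation, then refills a full magazine or the player's AmmoCount4Widget amount, depending on the character's IsLessThan flag.
; A GameInstance upgrade event swaps the mesh to a gold material.
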(event `/Game/ThirdPersonBP/Blueprints/Guns_Interface.Fire2`
  (params (ActorClass :type "Actor Object Reference"))
  (bind _ebbarrel_pistol (`self.EBBarrel_Pistol`))
  (bind _returnvalue (`EBBarrel.GetAmmoCount` _ebbarrel_pistol false))
  ;[1 1 1] Fire
  (if (>= _returnvalue 0)
    (`EBBarrel.Shoot` _ebbarrel_pistol true)
    (if (== _returnvalue 0)
      (`/Engine/EditorBlueprintResources/StandardMacros.DoOnce` false :!label _label
        (:`Completed`
          (`AudioComponent.Play` (`self.OutofAmmo_Sound`) 0.0)
          (`KismetSystemLibrary.Delay` 1.0)
          (goto _label :!via `Reset`))))))

(event `self.EBBarrel_Pistol.ShotFired`
  (`AudioComponent.Play` (`self.Gunshot_Pistol_Sound`) 0.0)
  (`ActorComponent.Activate` (`self.PistolShotFX`) true))

(event `/Game/ThirdPersonBP/Blueprints/Guns_Interface.UnFire2`
  (params (ActorClass :type "Actor Object Reference"))
  ;[1 1 1] Stop Firing
  (`EBBarrel.Shoot` (`self.EBBarrel_Pistol`) false))

(event `/Game/ThirdPersonBP/Blueprints/Guns_Interface.Reload2`
  (params (ActorClass :type "Actor Object Reference"))
  (bind _ebbarrel_pistol (`self.EBBarrel_Pistol`))
  (bind _asthird_person_char (cast `/Game/ThirdPersonBP/Blueprints/ThirdPersonChar` (`GameplayStatics.GetPlayerCharacter` 0) :!pure true))
  ;[1 1 1] Reload
  (set `EBBarrel.ShootingBlocked` true _ebbarrel_pistol)
  (`GameplayStatics.PlaySoundAtLocation` "/Game/MilitaryWeapSilver/Sound/Pistol/Wavs/Pistol_Reload03.Pistol_Reload03" (`SceneComponent.K2_GetComponentLocation` (`self.EBBarrel_Pistol`)) (struct) 1.0 1.0 0.0 null null null)
  (`SkeletalMeshComponent.PlayAnimation` (`self.PistolMesh`) "/Game/AnimStarterPack/Reload_Pistol.Reload_Pistol" false)
  (`KismetSystemLibrary.Delay` 1.7)
  (if (`/Game/ThirdPersonBP/Blueprints/ThirdPersonChar.isLessThan?` _asthird_person_char)
    (`EBBarrel.SetAmmo` _ebbarrel_pistol (`/Game/ThirdPersonBP/Blueprints/ThirdPersonChar.ammoCount4Widget` _asthird_person_char) true true false (`EBBarrel.Ammo` _ebbarrel_pistol))
    (set `EBBarrel.ShootingBlocked` false _ebbarrel_pistol)
    (else
      (`EBBarrel.SetAmmo` _ebbarrel_pistol 12 true true false (`EBBarrel.Ammo` _ebbarrel_pistol))
      (set `EBBarrel.ShootingBlocked` false _ebbarrel_pistol))))

(event `self.ReceiveBeginPlay`
  (bind _asmy_game_instance (cast `/Game/ThirdPersonBP/Blueprints/myGameInstance` (`GameplayStatics.GetGameInstance`)))
  (add `/Game/ThirdPersonBP/Blueprints/myGameInstance.Upgrade 3 DP` _asmy_game_instance (delegate `Upgrade 3 (GOLD)`)))

(event `Upgrade 3 (GOLD)`
  (`PrimitiveComponent.SetMaterial` (`self.PistolMesh`) 0 "/Game/MilitaryWeapSilver/Weapons/Materials/PistolGold.PistolGold"))

(fn `UserConstructionScript`)