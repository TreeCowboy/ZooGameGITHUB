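; Sniper rifle Blueprint that fires, stops firing and reloads through an EBBarrel ballistics component.
; Fire shoots when not reloading and ammo is at least zero, otherwise playing an out-of-ammo sound if not reloading; each shot triggers gunshot sound and FX.
; Reload blocks shooting during a timed delay, then resets ammo.
; IsReloading is never set here, and the reload sound and animation are disconnected.
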(event `/Game/ThirdPersonBP/Blueprints/Guns_Interface.Fire2`
  (params (ActorClass :type "Actor Object Reference"))
  (bind _ebbarrel_sniper (`self.EBBarrel_Sniper`))
  (bind _returnvalue (not (`self.IsReloading?`)))
  ;[1 1 1] Fire
  (if (and _returnvalue (>= (`EBBarrel.GetAmmoCount` _ebbarrel_sniper false) 0))
    (`EBBarrel.Shoot` _ebbarrel_sniper true)
    (elif _returnvalue
      (`AudioComponent.Play` (`self.OutOfAmmo_Sniper_Sound`) 0.0))))

(event `/Game/ThirdPersonBP/Blueprints/Guns_Interface.UnFire2`
  (params (ActorClass :type "Actor Object Reference"))
  ;[1 1 1] Stop Firing
  (`EBBarrel.Shoot` (`self.EBBarrel_Sniper`) false))

(event `/Game/ThirdPersonBP/Blueprints/Guns_Interface.Reload2`
  (params (ActorClass :type "Actor Object Reference"))
  (bind _ebbarrel_sniper (`self.EBBarrel_Sniper`))
  ;[1 1 1] Reload
  (set `EBBarrel.ShootingBlocked` true (`self.EBBarrel_Sniper`))
  (`KismetSystemLibrary.Delay` 2.2)
  (`EBBarrel.SetAmmo` _ebbarrel_sniper 4 false true false (`EBBarrel.Ammo` _ebbarrel_sniper))
  (set `EBBarrel.ShootingBlocked` false _ebbarrel_sniper))

(event `self.EBBarrel_Sniper.ShotFired`
  ;[1 1 1] Firing FX
  (`AudioComponent.Play` (`self.Gunshot_Sniper_Sound`) 0.0)
  (`ActorComponent.Activate` (`self.SniperFireFX`) true))

(fn `UserConstructionScript`)