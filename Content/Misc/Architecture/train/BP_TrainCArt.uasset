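; A train cart actor that rides along the spline of a referenced track.
; On BeginPlay it registers its MoveCart event with the game instance through AssignCartWithTrain.
; After a short delay, MoveCart plays a timeline scaled by Duration and starting at CartStartOffset.
; The timeline alpha maps to spline distance, setting location with a raised Z and rotation to match the track.
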(event `self.ReceiveBeginPlay`
  (add `/Game/ThirdPersonBP/Blueprints/myGameInstance.cartWithTrain` (cast `/Game/ThirdPersonBP/Blueprints/myGameInstance` (`GameplayStatics.GetGameInstance`) :!pure true) (delegate `MoveCart`)))

(event `MoveCart`
  (bind _trainspline (`/Game/Misc/Architecture/train/BP_TrainTrackPrecise.TrainSpline` (`self.trackRef`)))
  (bind _returnvalue (`KismetMathLibrary.Lerp` 0.0 (`SplineComponent.GetSplineLength` _trainspline) (`self.Alpha`)))
  (bind (_returnvalue_x _returnvalue_y _returnvalue_z) (`KismetMathLibrary.BreakVector` (`SplineComponent.GetLocationAtDistanceAlongSpline` _trainspline _returnvalue "World")))
  (`KismetSystemLibrary.Delay` 0.25)
  (`TimelineComponent.SetPlayRate` (`self.cartMove`) (/ 1.0 (`self.Duration`)))
  (`TimelineComponent.SetNewTime` (`self.cartMove`) (`self.cartStartOffset`))
  (bind (_direction _alpha) (`Timeline|cartMove`)
    (:`Update`
      (set `self.Alpha` _alpha)
      (`self.K2_SetActorLocationAndRotation` (`KismetMathLibrary.MakeVector` _returnvalue_x _returnvalue_y (+ _returnvalue_z 100.0)) (`SplineComponent.GetRotationAtDistanceAlongSpline` _trainspline _returnvalue "World")))))

(fn `UserConstructionScript`)