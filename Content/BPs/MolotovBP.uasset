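; Thrown-molotov actor that shatters and starts a fire on its first hit.
; A DoOnce on the Hit event plays a glass-break sound, damages the MolotovDM destructible mesh at the impact point to fracture it, and spawns a Molotov_Fire at the actor's location.
; The actor destroys itself after a delay, and the construction script is empty.
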(event `self.ReceiveHit`
  (params (MyComp :type "PrimitiveComponent Object Reference") (Other :type "Actor Object Reference") (OtherComp :type "PrimitiveComponent Object Reference") (bSelfMoved :type Boolean) (HitLocation :type "Vector Structure") (HitNormal :type "Vector Structure") (NormalImpulse :type "Vector Structure") (Hit :type "HitResult Structure (by ref)"))
  (bind (_bblockinghit _binitialoverlap _time _distance _location _impactpoint) (`GameplayStatics.BreakHitResult` Hit))
  (`/Engine/EditorBlueprintResources/StandardMacros.DoOnce` false
    (:`Completed`
      (`AudioComponent.Play` (`self.GlassBreakSound`) 0.46)
      (`DestructibleComponent.ApplyDamage` (`self.MolotovDM`) 100.0 _impactpoint _impactpoint 0.0)
      (`|SpawnActorFromClass` "/Game/BPs/Molotov_Fire.Molotov_Fire_C" (`KismetMathLibrary.MakeTransform` (`self.K2_GetActorLocation`)) "AlwaysSpawn" "OverrideRootScale" null null)
      (`KismetSystemLibrary.Delay` 10.0)
      (`self.K2_DestroyActor`))))

(fn `UserConstructionScript`)