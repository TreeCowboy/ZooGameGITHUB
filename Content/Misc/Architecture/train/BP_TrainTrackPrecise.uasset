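; BP_TrainTrackPrecise is a train track actor that builds its geometry along the TrainSpline.
; The construction script adds one spline mesh per section, with section length derived from the actor's X scale.
; Each mesh takes positions and tangents from the spline at its ends, with tangent size clamped to the section length.
; The event graph has no active logic.
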(fn `UserConstructionScript`
  (bind _returnvalue_x (`KismetMathLibrary.BreakVector` (`self.GetActorScale3D`)))
  (bind _trainspline (`self.TrainSpline`))
  (bind _trainspline_2 (`self.TrainSpline`))
  (set `self.SectionLength` (* _returnvalue_x 100.0))
  (for _index (range (+ (`KismetMathLibrary.FTrunc` (/ (`SplineComponent.GetSplineLength` (`self.TrainSpline`)) (`self.SectionLength`))) 1))
    (bind _returnvalue (`AddComponent|NODE_AddSplineMeshComponent-1`))
    (`SplineMeshComponent.SetForwardAxis` _returnvalue "X" true)
    (bind _returnvalue_2 (* _index (`self.SectionLength`)))
    (bind _returnvalue_3 (* (+ _index 1) (`self.SectionLength`)))
    (`SplineMeshComponent.SetStartAndEnd` _returnvalue (`SplineComponent.GetLocationAtDistanceAlongSpline` _trainspline _returnvalue_2 "Local") (`KismetMathLibrary.ClampVectorSize` (`SplineComponent.GetTangentAtDistanceAlongSpline` _trainspline _returnvalue_2 "Local") 0.0 (`self.SectionLength`)) (`SplineComponent.GetLocationAtDistanceAlongSpline` _trainspline_2 _returnvalue_3 "Local") (`KismetMathLibrary.ClampVectorSize` (`SplineComponent.GetTangentAtDistanceAlongSpline` _trainspline_2 _returnvalue_3 "Local") 0.0 (`self.SectionLength`)) true)))