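; BP_Train is a train actor that travels along the spline of a referenced track actor.
; If activated on BeginPlay, it runs the TrainMover timeline with play rate scaled by Duration and a configurable start offset.
; Each update maps the timeline alpha to distance along TrainSpline and sets the actor's world location and rotation to match.
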(event `self.ReceiveBeginPlay`
  (if (`self.activateTrain`)
    (`self.MoveTrain`)))

(event `MoveTrain`
  (bind _trainspline (`/Game/Misc/Architecture/train/BP_TrainTrack.TrainSpline` (`self.trackReference`)))
  (bind _returnvalue (`KismetMathLibrary.Lerp` 0.0 (`SplineComponent.GetSplineLength` _trainspline) (`self.Alpha`)))
  (`TimelineComponent.SetPlayRate` (`self.trainMover`) (/ 1.0 (`self.Duration`)))
  (`TimelineComponent.SetNewTime` (`self.trainMover`) (`self.Train Start Offset`))
  (bind (_direction _alpha) (`Timeline|trainMover`)
    (:`Update`
      (set `self.Alpha` _alpha)
      (`self.K2_SetActorLocationAndRotation` (`SplineComponent.GetLocationAtDistanceAlongSpline` _trainspline _returnvalue "World") (`SplineComponent.GetRotationAtDistanceAlongSpline` _trainspline _returnvalue "World")))))

(fn `UserConstructionScript`)