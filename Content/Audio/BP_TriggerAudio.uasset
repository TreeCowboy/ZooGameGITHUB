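; BP_TriggerAudio is a trigger volume that toggles its own 2D sound when the player character enters its box.
; BeginPlay creates a persistent audio component and caches all BP_TriggerAudio actors.
; Overlap loops over that array but only uses this actor's component, fading it in or out by IsPlayingSound.
; The flag flips after a Delay inside the loop.
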(event `self.ReceiveBeginPlay`
  (bind _outactors (`GameplayStatics.GetAllActorsOfClass` "BP_TriggerAudio_C"))
  (set `self.Trigger Audio Boxes` _outactors)
  (bind _returnvalue (`GameplayStatics.CreateSound2D` (`self.Sound`) 1.0 1.0 0.0 null false false))
  (set `self.AudioComponent` _returnvalue))

(event `self.Box.OnComponentBeginOverlap`
  (params (OverlappedComponent :type "PrimitiveComponent Object Reference") (OtherActor :type "Actor Object Reference") (OtherComp :type "PrimitiveComponent Object Reference") (OtherBodyIndex :type Integer) (bFromSweep :type Boolean) (SweepResult :type "HitResult Structure (by ref)"))
  (bind _audiocomponent (`self.AudioComponent`))
  (if (== OtherActor (`GameplayStatics.GetPlayerCharacter` 0))
    (for _ (`self.Trigger Audio Boxes`)
      (if (not (`self.isPlayingSound?`))
        (`AudioComponent.FadeIn` _audiocomponent 0.0 1.0 0.0 "Linear")
        (`KismetSystemLibrary.Delay` 2.0)
        (set `self.isPlayingSound?` true)
        (else
          (`AudioComponent.FadeOut` _audiocomponent 2.0 0.0 "Linear")
          (`KismetSystemLibrary.Delay` 2.0)
          (set `self.isPlayingSound?` false))))))

(fn `UserConstructionScript`)