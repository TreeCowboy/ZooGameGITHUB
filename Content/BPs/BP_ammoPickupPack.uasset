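; Ammo pickup pack that notifies the player through AmmoPickupMessage on overlap, plays a pickup sound and destroys itself.
; The construction script picks the mesh from weapon flags on myGameInstance, with the grenade flag mapping to the pistol mesh.
; The pickup sound is always the sniper rifle's, whatever mesh is shown.
; BeginPlay assigns the collision component a custom object channel, and only player character 0 triggers the pickup.
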(event `self.ReceiveBeginPlay`
  (`PrimitiveComponent.SetCollisionObjectType` (`self.ammoCollision`) "ECC_GameTraceChannel3"))

(event `self.ammoCollision.OnComponentBeginOverlap`
  (params (OverlappedComponent :type "PrimitiveComponent Object Reference") (OtherActor :type "Actor Object Reference") (OtherComp :type "PrimitiveComponent Object Reference") (OtherBodyIndex :type Integer) (bFromSweep :type Boolean) (SweepResult :type "HitResult Structure (by ref)"))
  (if (== OtherActor (`GameplayStatics.GetPlayerCharacter` 0))
    (message `/Game/ThirdPersonBP/Blueprints/ammoInterface.ammoPickup` OtherActor)
    (`GameplayStatics.SpawnSoundAtLocation` "/Game/MilitaryWeapSilver/Sound/SniperRifle/Wavs/SniperRifle_AmmoPickup.SniperRifle_AmmoPickup" SweepResult_Location (struct) 1.0 1.0 0.0 null null)
    (`self.K2_DestroyActor`)))

(fn `UserConstructionScript`
  (bind _staticmesh (`self.StaticMesh`))
  (bind _asmy_game_instance (cast `/Game/ThirdPersonBP/Blueprints/myGameInstance` (`GameplayStatics.GetGameInstance`)))
  (if (`/Game/ThirdPersonBP/Blueprints/myGameInstance.IsGrenadGI` _asmy_game_instance)
    (`StaticMeshComponent.SetStaticMesh` _staticmesh "/Game/MilitaryWeapSilver/Pickups/Pistol_Pickup.Pistol_Pickup")
    (elif (`/Game/ThirdPersonBP/Blueprints/myGameInstance.isAssaultRifleGI` _asmy_game_instance)
      (`StaticMeshComponent.SetStaticMesh` _staticmesh "/Game/MilitaryWeapSilver/Pickups/AssaultRifle_Pickup.AssaultRifle_Pickup")
      (elif (`/Game/ThirdPersonBP/Blueprints/myGameInstance.IsSniperGI` _asmy_game_instance)
        (`StaticMeshComponent.SetStaticMesh` _staticmesh "/Game/MilitaryWeapSilver/Pickups/SniperRifle_Pickup.SniperRifle_Pickup")
        (elif (`/Game/ThirdPersonBP/Blueprints/myGameInstance.IsShotgunGI` _asmy_game_instance)
          (`StaticMeshComponent.SetStaticMesh` _staticmesh "/Game/MilitaryWeapSilver/Pickups/Shotgun_Pickup.Shotgun_Pickup"))))))