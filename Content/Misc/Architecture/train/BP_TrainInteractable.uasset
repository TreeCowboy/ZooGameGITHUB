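; Interactable train actor that travels along a referenced track's spline and deals massive damage to whatever it hits.
; BeginPlay binds the move event to the inherited interaction event, which plays a timeline scaled by Duration from TrainStartOffset to set location and rotation by spline distance.
; Hits send a damage message with the impulse and play a recording; IsWhistle is set true just before its check, so it never gates the sound.
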(event `self.ReceiveBeginPlay`
  (add `self.DoEvent` (delegate `MoveTrain_Interact`)))

(event `MoveTrain_Interact`
  (bind _trainspline (`/Game/Misc/Architecture/train/BP_TrainTrackPrecise.TrainSpline` (`self.trackRef`)))
  (bind _returnvalue (`KismetMathLibrary.Lerp` 0.0 (`SplineComponent.GetSplineLength` _trainspline) (`self.Alpha`)))
  ;[1 1 1] Move Train
  (`TimelineComponent.SetPlayRate` (`self.TrainMove`) (/ 1.0 (`self.Duration`)))
  (`TimelineComponent.SetNewTime` (`self.TrainMove`) (`self.trainStartOffset`))
  (bind (_direction _alpha) (`Timeline|TrainMove`)
    (:`Update`
      (set `self.Alpha` _alpha)
      (`self.K2_SetActorLocationAndRotation` (`SplineComponent.GetLocationAtDistanceAlongSpline` _trainspline _returnvalue "World") (`SplineComponent.GetRotationAtDistanceAlongSpline` _trainspline _returnvalue "World")))))

(event `self.ReceiveHit`
  (params (MyComp :type "PrimitiveComponent Object Reference") (Other :type "Actor Object Reference") (OtherComp :type "PrimitiveComponent Object Reference") (bSelfMoved :type Boolean) (HitLocation :type "Vector Structure") (HitNormal :type "Vector Structure") (NormalImpulse :type "Vector Structure") (Hit :type "HitResult Structure (by ref)"))
  ;[1 1 1] Train Impact
  (message `/Game/ThirdPersonBP/Blueprints/Shootables_Interface.DoDamage` Other NormalImpulse HitLocation 500000.0 "None")
  (set `self.isWhistle?` true)
  (if (`self.isWhistle?`)
    (`|ExecutionSequence`
      (:`then_0`
        (`GameplayStatics.PlaySoundAtLocation` "/Game/Misc/Architecture/train/Recording.Recording" HitLocation (struct) 1.0 1.0 0.0 null null null))
      (:`then_1`
        (set `self.isWhistle?` false)))))

(fn `UserConstructionScript`
  (`parent.UserConstructionScript`))