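; Assault rifle weapon Blueprint that handles firing, stopping and reloading through an EBBarrel ballistics component.
; Fire starts shooting unless reloading, with a DoOnce and one-second delay throttling the out-of-ammo sound.
; The barrel's ShotFired event triggers gunshot audio and firing effects.
; Reload plays an animation, waits, then refills a full magazine or the player character's remaining ammo, depending on its IsLessThan flag.
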(event `/Game/ThirdPersonBP/Blueprints/Guns_Interface.Fire2`
  (params (ActorClass :type "Actor Object Reference"))
  (bind _ebbarrel_assault (`self.EBBarrel_Assault`))
  (bind _returnvalue (`EBBarrel.GetAmmoCount` _ebbarrel_assault false))
  ;[1 1 1] Fire
  (if (`self.IsReloading?`)
    _
    (elif (>= _returnvalue 0)
      (`EBBarrel.Shoot` _ebbarrel_assault true)
      (if (== _returnvalue 0)
        (`/Engine/EditorBlueprintResources/StandardMacros.DoOnce` false :!label _label
          (:`Completed`
            (`AudioComponent.Play` (`self.OutofAmmo_Sound`) 0.0)
            (`KismetSystemLibrary.Delay` 1.0)
            (goto _label :!via `Reset`)))))))

(event `/Game/ThirdPersonBP/Blueprints/Guns_Interface.UnFire2`
  (params (ActorClass :type "Actor Object Reference"))
  ;[1 1 1] Stop Firing
  (`EBBarrel.Shoot` (`self.EBBarrel_Assault`) false))

(event `self.EBBarrel_Assault.ShotFired`
  ;[1 1 1] Effects from Firing
  (`AudioComponent.Play` (`self.GunShot_AssaultRifle_Sound`) 0.0)
  (`ActorComponent.Activate` (`self.FireEffect_AR`) true))

(event `/Game/ThirdPersonBP/Blueprints/Guns_Interface.Reload2`
  (params (ActorClass :type "Actor Object Reference"))
  (bind _ebbarrel_assault (`self.EBBarrel_Assault`))
  (bind _asthird_person_char (cast `/Game/ThirdPersonBP/Blueprints/ThirdPersonChar` (`GameplayStatics.GetPlayerCharacter` 0) :!pure true))
  ;[1 1 1] Reload
  (`SkeletalMeshComponent.PlayAnimation` (`self.SkeletalMesh`) "/Game/MilitaryWeapSilver/Weapons/Animations/Reload_Rifle_Ironsights_W.Reload_Rifle_Ironsights_W" false)
  (`KismetSystemLibrary.Delay` 2.2)
  (if (`/Game/ThirdPersonBP/Blueprints/ThirdPersonChar.isLessThan?` _asthird_person_char)
    (`EBBarrel.SetAmmo` _ebbarrel_assault (`/Game/ThirdPersonBP/Blueprints/ThirdPersonChar.ammoCount4Widget` _asthird_person_char) true true false (`EBBarrel.Ammo` _ebbarrel_assault))
    (set `EBBarrel.ShootingBlocked` false _ebbarrel_assault)
    (set `self.IsReloading?` false)
    (else
      (`EBBarrel.SetAmmo` _ebbarrel_assault 16 true true false (`EBBarrel.Ammo` _ebbarrel_assault))
      (set `EBBarrel.ShootingBlocked` false _ebbarrel_assault)
      (set `self.IsReloading?` false))))

(fn `UserConstructionScript`)