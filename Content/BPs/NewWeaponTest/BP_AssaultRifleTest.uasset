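; BP_AssaultRifleTest is a test assault rifle that handles firing, stopping and reloading through an EBBarrel ballistics component.
; Firing starts the barrel shooting and runs a timeline that copies ammo count to ThirdPersonChar for the ammo widget.
; An empty magazine plays a throttled out-of-ammo sound, while reloading refills the magazine and blocks firing during a delay.
; The barrel's ShotFired event triggers the gunshot sound and muzzle effect.
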(event `Reload`
  (bind _ebbarrel_assaulttest (`self.EBBarrel_AssaultTest`))
  ;[1 1 1] Reloading
  (if (and (not (`self.IsReloading?`)) (< (`EBBarrel.GetAmmoCount` _ebbarrel_assaulttest true) 16))
    (`EBBarrel.SetAmmo` (`self.EBBarrel_AssaultTest`) 16 true true false (`EBBarrel.Ammo` _ebbarrel_assaulttest))
    (`AudioComponent.Play` (`self.Reload_Test`) 0.0)
    (set `self.isReloading?` true)
    (`KismetSystemLibrary.Delay` 3.4)
    (set `self.isReloading?` false)))

(event `FiringGun`
  (bind _ebbarrel_assaulttest (`self.EBBarrel_AssaultTest`))
  ;[1 1 1] Firing Weapon
  (if (> (`EBBarrel.GetAmmoCount` _ebbarrel_assaulttest false) 0)
    (if (not (`self.IsReloading?`))
      (`EBBarrel.Shoot` _ebbarrel_assaulttest true)
      ;[1 1 1] Updates Ammo Count for Ammo Widget
      (`Timeline|Timeline_0` :!label _label
        (:`Update`
          _)
        (:`BC Track`
          _))
      (set `/Game/ThirdPersonBP/Blueprints/ThirdPersonChar.ammoCount4Widget` (`EBBarrel.GetAmmoCount` (`self.EBBarrel_AssaultTest`) false) (cast `/Game/ThirdPersonBP/Blueprints/ThirdPersonChar` (`GameplayStatics.GetPlayerCharacter` 0) :!pure true)))
    (else
      (`/Engine/EditorBlueprintResources/StandardMacros.DoOnce` false :!label _label_2
        (:`Completed`
          (`AudioComponent.Play` (`self.OOA_Test`) 0.0)
          (`KismetSystemLibrary.Delay` 1.0)
          (goto _label_2 :!via `Reset`))))))

(event `StopFiring`
  ;[1 1 1] Stop Shooting
  (`|ExecutionSequence`
    (:`then_0`
      (`EBBarrel.Shoot` (`self.EBBarrel_AssaultTest`) false))
    (:`then_1`
      (goto _label :!via `SetNewTime`))
    (:`then_2`
      (goto _label :!via `Stop`))))

(event `self.EBBarrel_AssaultTest.ShotFired`
  ;[1 1 1] Effects from Firing
  (`AudioComponent.Play` (`self.Gunshot_Test`) 0.0)
  (`ActorComponent.Activate` (`self.fireEffect_Test`) true))

(fn `UserConstructionScript`
  (`parent.UserConstructionScript`))