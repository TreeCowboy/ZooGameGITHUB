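; Player shotgun Blueprint that handles interface-driven firing and reloading through an EBBarrel component, reading and writing ammo state on ThirdPersonChar.
; Each shot triggers sound, muzzle effect, a timed-life shell casing and random camera recoil.
; Reload blocks shooting for a duration scaled by missing shells, using a DoN and retriggerable-delay loop for per-shell sounds.
; Game instance dispatchers apply upgrades: larger capacity, or gold material with added fire ammo.
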(event `numAnimationsEvent`
  (bind _asthird_person_char (cast `/Game/ThirdPersonBP/Blueprints/ThirdPersonChar` (`GameplayStatics.GetPlayerCharacter` 0) :!pure true))
  (bind _returnvalue (- (`/Game/ThirdPersonBP/Blueprints/ThirdPersonChar.ammoPack` _asthird_person_char) (`/Game/ThirdPersonBP/Blueprints/ThirdPersonChar.ammoCount4Widget` _asthird_person_char)))
  (bind _output_get (set `/Game/ThirdPersonBP/Blueprints/ThirdPersonChar.shottyDuration` (+ 1.84 (* _returnvalue 0.4)) (cast `/Game/ThirdPersonBP/Blueprints/ThirdPersonChar` (`GameplayStatics.GetPlayerCharacter` 0) :!pure true)))
  (`KismetSystemLibrary.Delay` 1.84)
  (bind _counter (`/Engine/EditorBlueprintResources/StandardMacros.Do N` _returnvalue :!label _label)
    (:`Exit`
      (`GameplayStatics.SpawnSound2D` "/Game/MilitaryWeapSilver/Sound/Shotgun/Cues/Shotgun_Reload_In_Cue.Shotgun_Reload_In_Cue" 1.0 1.0 0.0 null)
      (if (== _counter _returnvalue)
        (`KismetSystemLibrary.PrintString` "done")
        (bind _output_get_2 (set `self.doneReloading?` true))
        (set `/Game/ThirdPersonBP/Blueprints/myGameInstance.isDoneReloadingGI` _output_get_2 (cast `/Game/ThirdPersonBP/Blueprints/myGameInstance` (`GameplayStatics.GetGameInstance`) :!pure true))
        (goto _label :!via `Reset`)
        (else
          (`KismetSystemLibrary.PrintString` "not done")
          (`KismetSystemLibrary.RetriggerableDelay` 0.2)
          (goto _label))))))

(event `Reload`
  (bind _ebbarrel_shotty (`self.EBBarrel_Shotty`))
  (bind _asthird_person_char (cast `/Game/ThirdPersonBP/Blueprints/ThirdPersonChar` (`GameplayStatics.GetPlayerCharacter` 0) :!pure true))
  (bind _ammo (`EBBarrel.Ammo` _ebbarrel_shotty))
  ;[1 1 1] Reload Event
  (if (and (not (`self.IsReloading?`)) (< (`EBBarrel.GetAmmoCount` _ebbarrel_shotty false) 6))
    (set `EBBarrel.ShootingBlocked` true _ebbarrel_shotty)
    (set `self.IsReloading?` true)
    (`self.numAnimationsEvent`)
    (`KismetSystemLibrary.Delay` (stale `numAnimationsEvent` _output_get))
    (if (`/Game/ThirdPersonBP/Blueprints/ThirdPersonChar.isLessThan?` _asthird_person_char)
      (`EBBarrel.SetAmmo` _ebbarrel_shotty (`/Game/ThirdPersonBP/Blueprints/ThirdPersonChar.ammoCount4Widget` _asthird_person_char) true true false _ammo)
      (set `EBBarrel.ShootingBlocked` false _ebbarrel_shotty)
      (set `self.IsReloading?` false)
      (else
        (`EBBarrel.SetAmmo` _ebbarrel_shotty (`self.Ammo Count`) true true false _ammo)
        (set `EBBarrel.ShootingBlocked` false _ebbarrel_shotty)
        (set `self.IsReloading?` false)))))

(event `FiringGun`
  (bind _ebbarrel_shotty (`self.EBBarrel_Shotty`))
  (bind _returnvalue (`EBBarrel.GetAmmoCount` _ebbarrel_shotty true))
  ;[1 1 1] Fire Event
  (if (>= _returnvalue 0)
    (if (not (`self.IsReloading?`))
      (`EBBarrel.Shoot` _ebbarrel_shotty true)
      (if (== _returnvalue 0)
        (`AudioComponent.Play` (`self.OutOfAmmo_Shotty`) 0.0)))))

(event `self.UnFire2`
  (params (ActorClass :type "Actor Object Reference"))
  ;[1 1 1] Interface Calls
  (`self.StopFiring`))

(event `StopFiring`
  ;[1 1 1] Stop Firing
  (`EBBarrel.Shoot` (`self.EBBarrel_Shotty`) false))

(event `self.Fire2`
  (params (ActorClass :type "Actor Object Reference"))
  ;[1 1 1] Interface Calls
  (`self.FiringGun`))

(event `self.Reload2`
  (params (ActorClass :type "Actor Object Reference"))
  ;[1 1 1] Interface Calls
  (`self.Reload`))

(event `self.EBBarrel_Shotty.ShotFired`
  (`AudioComponent.Play` (`self.Shotgun_Fire_Sound`) 0.0)
  (`ActorComponent.Activate` (`self.FireEffect_Shotty`) true)
  ;[1 1 1] Release Shell
  (bind _returnvalue (`|SpawnActorFromClass` "/Game/BPs/Shell.Shell_C" (`KismetMathLibrary.MakeTransform` (+ (`SceneComponent.K2_GetComponentLocation` (`self.Shotgun`)) (-15.0 -15.0 -60.0)) (`KismetMathLibrary.RandomRotator` true) (0.01 0.01 0.01)) "AdjustIfPossibleButDontSpawnIfColliding" "OverrideRootScale" null null))
  (`self.SetLifeSpan` _returnvalue 15.0)
  ;[1 1 1] Recoil
  (bind _asthird_person_char (cast `/Game/ThirdPersonBP/Blueprints/ThirdPersonChar` (`GameplayStatics.GetPlayerCharacter` 0)))
  (`self.Recoil` _asthird_person_char (`KismetMathLibrary.RandomFloatInRange` -1.0 -0.4) (`KismetMathLibrary.RandomFloatInRange` -0.3 0.3)))

(event `self.ReceiveBeginPlay`
  ;[1 1 1] UPGRADES
  (bind _asmy_game_instance (cast `/Game/ThirdPersonBP/Blueprints/myGameInstance` (`GameplayStatics.GetGameInstance`)))
  (add `/Game/ThirdPersonBP/Blueprints/myGameInstance.Upgrade 3 DP` _asmy_game_instance (delegate `Upgrade3(GOLD)`))
  (add `/Game/ThirdPersonBP/Blueprints/myGameInstance.Upgrade 2 DP` _asmy_game_instance (delegate `Upgrade 2`)))

(event `Upgrade 2`
  (bind _asthird_person_char (cast `/Game/ThirdPersonBP/Blueprints/ThirdPersonChar` (`GameplayStatics.GetPlayerCharacter` 0) :!pure true))
  ;[1 1 1] UPGRADES
  (set `EBBarrel.CycleAmmoCount` 9 (`self.EBBarrel_Shotty`))
  (set `self.Ammo Count` 9)
  (set `/Game/ThirdPersonBP/Blueprints/ThirdPersonChar.ammoPack` 9 _asthird_person_char)
  (set `/Game/ThirdPersonBP/Blueprints/ThirdPersonChar.ammoCount4Widget` 9 _asthird_person_char))

(event `Upgrade3(GOLD)`
  (bind _ammo (`EBBarrel.Ammo` (`self.EBBarrel_Shotty`)))
  ;[1 1 1] UPGRADES
  (`PrimitiveComponent.SetMaterial` (`self.Shotgun`) 0 "/Game/MilitaryWeapSilver/Weapons/Materials/ShotgunGold.ShotgunGold")
  (`KismetArrayLibrary.Array_Add` _ammo "/Game/BPs/ShotgunBullet_Fire.ShotgunBullet_Fire_C")
  (`KismetArrayLibrary.Array_Add` _ammo "/Game/BPs/shotgunBullet.shotgunBullet_C")
  (`KismetArrayLibrary.Array_Add` _ammo "/Game/BPs/shotgunBullet.shotgunBullet_C"))

(fn `numAnimations`
  (bind _shotgun (`self.Shotgun`))
  (bind _asthird_person_char (cast `/Game/ThirdPersonBP/Blueprints/ThirdPersonChar` (`GameplayStatics.GetPlayerCharacter` 0) :!pure true))
  (for _ (range 1 (+ (- (`/Game/ThirdPersonBP/Blueprints/ThirdPersonChar.ammoPack` _asthird_person_char) (`/Game/ThirdPersonBP/Blueprints/ThirdPersonChar.ammoCount4Widget` _asthird_person_char)) 1))
    (`SkeletalMeshComponent.PlayAnimation` _shotgun "/Game/MilitaryWeapSilver/Weapons/Animations/Reload_Shotgun_1Shell.Reload_Shotgun_1Shell" false))
  (`SkeletalMeshComponent.PlayAnimation` _shotgun "/Game/MilitaryWeapSilver/Weapons/Animations/Reload_Shotgun_Finished.Reload_Shotgun_Finished" false))

(fn `UserConstructionScript`)